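; An actor that repeatedly spawns NPCs at its root location while a countdown value is within a short window.
; BeginPlay runs a Delay-based polling loop that calls SpawnNPC whenever CountDown is above zero and below a small threshold, then waits a random interval.
; Outside that window it rechecks at a short fixed interval, and nothing in this graph changes CountDown.
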(event `Spawn NPC`
  (`|SpawnActorFromClass` "/Game/Characters/AI/NPC.NPC_C" (`KismetMathLibrary.Conv_VectorToTransform` (`SceneComponent.K2_GetComponentLocation` (`self.DefaultSceneRoot`))) "Undefined" "MultiplyWithRoot" null null))

(event `self.ReceiveBeginPlay`
  (bind _count_down (`self.Count Down`))
  (if (> _count_down 0.0) :!label _label
    (if (< _count_down 5.0)
      (`self.Spawn NPC`)
      (`KismetSystemLibrary.Delay` (`KismetMathLibrary.RandomFloatInRange` 0.5 2.0))
      (goto _label)
      (else
        _)))
  (`KismetSystemLibrary.Delay` 0.2)
  (goto _label))

(fn `UserConstructionScript`)