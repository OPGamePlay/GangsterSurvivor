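; Coin_cube_BP is a collectible coin that spins and bobs up and down in the world.
; A self-looping BeginPlay chain using DelayUntilNextTick drives the motion in fixed per-frame steps, so speed depends on frame rate, and a step counter flips the vertical direction.
; Overlapping its Box with BP_ThirdPersonCharacter adds that character's CoinMultiplier to its CoinValue, destroys the coin and plays a pickup sound.
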(event `self.ReceiveBeginPlay`
  (set `self.max_up` 200)
  (set `self.updown_direction` false)
  (`self.K2_AddActorWorldRotation` (struct :`Yaw` 1.0) :!label _label)
  (if (`self.updown_direction`)
    (`self.K2_AddActorLocalOffset` (`KismetMathLibrary.MakeVector` 0.0 0.0 0.2))
    (bind _output_get (set `self.current_offset` (+ (`self.current_offset`) 1)))
    (if (>= _output_get (`self.max_up`))
      (set `self.updown_direction` false))
    (else
      (`self.K2_AddActorLocalOffset` (`KismetMathLibrary.MakeVector` 0.0 0.0 -0.2))
      (bind _output_get_2 (set `self.current_offset` (- (`self.current_offset`) 1)))
      (if (<= _output_get_2 0)
        (set `self.updown_direction` true))))
  (`KismetSystemLibrary.DelayUntilNextTick`)
  (goto _label))

(event `self.Box.OnComponentBeginOverlap`
  (params (OverlappedComponent :type "PrimitiveComponent Object Reference") (OtherActor :type "Actor Object Reference") (OtherComp :type "PrimitiveComponent Object Reference") (OtherBodyIndex :type Integer) (bFromSweep :type Boolean) (SweepResult :type "HitResult Structure (by ref)"))
  ;[1 1 1] Coin_pickup
  (bind _asbp_third_person_character (cast `/Game/Characters_BPs/MainCharater_BP/Blueprints/BP_ThirdPersonCharacter` OtherActor))
  (set `/Game/Characters_BPs/MainCharater_BP/Blueprints/BP_ThirdPersonCharacter.CoinValue` (+ (`/Game/Characters_BPs/MainCharater_BP/Blueprints/BP_ThirdPersonCharacter.CoinValue` _asbp_third_person_character) (`/Game/Characters_BPs/MainCharater_BP/Blueprints/BP_ThirdPersonCharacter.Coin Multiplier` _asbp_third_person_character)) _asbp_third_person_character)
  (`self.K2_DestroyActor`)
  (`GameplayStatics.PlaySound2D` "/Game/Props/Coin_cube/money-pickup-2-89563.money-pickup-2-89563" 1.0 1.0 0.0 null null))

(fn `UserConstructionScript`)