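; NPC spawner actor that spawns NPCs at random XY offsets around itself, at a fixed world height, while a player is nearby.
; When active, a player-tagged actor entering the Trigger starts a looping SpawnNPC timer with an interval randomized once per start.
; Leaving the trigger clears that timer after a short delay.
; A separate Spawner event polls IsActive for randomly paced continuous spawning, but nothing here calls it.
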(event `Spawn NPC`
  (bind (_returnvalue_x _returnvalue_y) (`KismetMathLibrary.BreakVector` (`self.K2_GetActorLocation`)))
  (bind _output_get (set `self.SpawnLocation` (`KismetMathLibrary.MakeVector` (+ _returnvalue_x (`KismetMathLibrary.RandomFloatInRange` -2000.0 2000.0)) (+ _returnvalue_y (`KismetMathLibrary.RandomFloatInRange` -2000.0 2000.0)) 200.0)))
  (`|SpawnActorFromClass` "/Game/Characters_BPs/AI/NPC.NPC_C" (`KismetMathLibrary.Conv_VectorToTransform` _output_get) "Undefined" "MultiplyWithRoot" null null)
  (`KismetSystemLibrary.PrintString` "success spawn"))

(event `Spawner`
  (if (`self.IsActive`) :!label _label
    (`self.Spawn NPC`)
    (`KismetSystemLibrary.Delay` (`KismetMathLibrary.RandomFloatInRange` 0.5 5.0))
    (goto _label)
    (else
      (`KismetSystemLibrary.Delay` 0.2)
      (goto _label))))

(event `Stop Spawn`
  (`KismetSystemLibrary.Delay` 2.0)
  (`KismetSystemLibrary.K2_ClearAndInvalidateTimerHandle` (stale `self.Trigger.OnComponentBeginOverlap` _returnvalue))
  (`KismetSystemLibrary.PrintString` "stop spawn"))

(event `self.Trigger.OnComponentBeginOverlap`
  (params (OverlappedComponent :type "PrimitiveComponent Object Reference") (OtherActor :type "Actor Object Reference") (OtherComp :type "PrimitiveComponent Object Reference") (OtherBodyIndex :type Integer) (bFromSweep :type Boolean) (SweepResult :type "HitResult Structure (by ref)"))
  (if (and (`self.IsActive`) (`self.ActorHasTag` OtherActor "Player"))
    (bind _returnvalue (`KismetSystemLibrary.K2_SetTimerDelegate` (delegate `Spawn NPC`) (`KismetMathLibrary.RandomFloatInRange` 0.2 1.0) true))))

(event `self.Trigger.OnComponentEndOverlap`
  (params (OverlappedComponent :type "PrimitiveComponent Object Reference") (OtherActor :type "Actor Object Reference") (OtherComp :type "PrimitiveComponent Object Reference") (OtherBodyIndex :type Integer))
  (if (`self.ActorHasTag` OtherActor "Player")
    (`self.Stop Spawn`)))

(fn `UserConstructionScript`)