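; BP_AI_Bird is an AI bird that homes in on the player and can drop a run of bombs.
; On BeginPlay it sets the third-person character's mesh as the homing target of its ProjectileMovement.
; StartBombSequence, not called within this Blueprint, resets a counter and runs a self-calling delay event that spawns five Bombs a second apart at the Spwan component.
; A separate bombcount/spwanbomb path has no spawn class set.
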(event `StartBombSequence`
  (set `self.Count` 0.0)
  (`self.dropdelay`))

(event `dropdelay`
  (if (< (`self.Count`) 5.0)
    (bind _result (`/Engine/EditorBlueprintResources/StandardMacros.IncrementFloat` (`self.Count`))
      (:`  `
        (set `self.Count` _result)
        (`|SpawnActorFromClass` "/Game/Props/Bomb.Bomb_C" (`KismetMathLibrary.MakeTransform` (`SceneComponent.K2_GetComponentLocation` (`self.Spwan`))) "Undefined" "MultiplyWithRoot" null null)
        (`KismetSystemLibrary.Delay` 1.0)
        (`self.dropdelay`)))))

(event `bombcount`
  (set `self.Count` (`self.Count`))
  (`self.spwanbomb`))

(event `spwanbomb`
  (`|SpawnActorFromClass` "/Game/Props/Bomb.Bomb_C" (`KismetMathLibrary.MakeTransform` (`SceneComponent.K2_GetComponentLocation` (`self.Spwan`))) "Undefined" "MultiplyWithRoot" null null))

(event `self.ReceiveBeginPlay`
  (bind _asbp_third_person_character (cast `/Game/Characters_BPs/MainCharater_BP/Blueprints/BP_ThirdPersonCharacter` (`GameplayStatics.GetPlayerCharacter` 0)))
  (set `ProjectileMovementComponent.HomingTargetComponent` (`Character.Mesh` _asbp_third_person_character) (`self.ProjectileMovement`)))

(fn `UserConstructionScript`)