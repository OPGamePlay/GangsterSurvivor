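; Pistol weapon actor that the third-person character picks up by proximity and that then auto-fires at nearby NPCs.
; While unowned it checks distance on Tick and claims a slot in the character's Weapons array if one is free.
; Once owned it orbits the character by slot angle and yaws toward the closest NPC in range.
; A Delay loop from BeginPlay repeatedly spawns Bullets along the muzzle rotation, with lifetime derived from range and speed.
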(event `self.ReceiveBeginPlay`
  (bind _guntest (`self.guntest`))
  (bind _speed (`self.Speed`))
  (if (and (`self.Owned`) (`self.closest_NPC_Exist`)) :!label _label
    (for _ (range 2)
      (bind _returnvalue (`|SpawnActorFromClass` "/Game/MyPackage/weapon/bullet.bullet_C" (`KismetMathLibrary.MakeTransform` (`SceneComponent.K2_GetComponentLocation` _guntest)) "Undefined" "MultiplyWithRoot" null null))
      (`/Game/MyPackage/weapon/bullet.init_bullet` _returnvalue (`KismetMathLibrary.MakeRotator` (.roll (`SceneComponent.K2_GetComponentRotation` _guntest)) (.pitch (`SceneComponent.K2_GetComponentRotation` _guntest)) (.yaw (`SceneComponent.K2_GetComponentRotation` _guntest))) (/ (`self.Range`) _speed) _speed (`self.Damage`) (`self.Accuracy`)))
    (`KismetSystemLibrary.Delay` 0.1)
    (goto _label)
    (else
      (`KismetSystemLibrary.Delay` 0.1)
      (goto _label))))

(event `self.ReceiveTick`
  (params (DeltaSeconds :type "Float (single-precision)"))
  (if (`self.Owned`)
    (`self.follow main charater`)
    (`self.Aim Angle update`)
    (else
      (`self.Check Distance`))))

(event `Check Distance`
  (bind _outactors (`GameplayStatics.GetAllActorsOfClass` "/Game/ThirdPerson/Blueprints/BP_ThirdPersonCharacter.BP_ThirdPersonCharacter_C"))
  (for _array_element _outactors
    (if (< (`self.GetDistanceTo` _array_element) 200.0)
      (if (< (`KismetArrayLibrary.Array_Length` (`/Game/ThirdPerson/Blueprints/BP_ThirdPersonCharacter.Weapons` _array_element)) (`/Game/ThirdPerson/Blueprints/BP_ThirdPersonCharacter.MaxWeapons` _array_element))
        (set `self.Owned` true)
        (bind _weapons (`/Game/ThirdPerson/Blueprints/BP_ThirdPersonCharacter.Weapons` _array_element))
        (bind _returnvalue (`KismetArrayLibrary.Array_Add` _weapons (`self.Name`)))
        (set `self.slot` (`KismetMathLibrary.Conv_IntToDouble` _returnvalue))
        (for _array_element_2 _weapons
          (`KismetSystemLibrary.PrintString` _array_element_2))
        (`KismetSystemLibrary.PrintString` "ok")))))

(event `follow main charater`
  (bind _weapondisplayradius (`self.WeaponDisplayRadius`))
  (bind _returnvalue (`GameplayStatics.GetActorOfClass` "/Game/ThirdPerson/Blueprints/BP_ThirdPersonCharacter.BP_ThirdPersonCharacter_C"))
  (bind _returnvalue_2 (* (/ (+ (`self.slot`) 1.0) (`KismetMathLibrary.Conv_IntToDouble` (`KismetArrayLibrary.Array_Length` (`/Game/ThirdPerson/Blueprints/BP_ThirdPersonCharacter.Weapons` (stale `Check Distance` _array_element))))) 360.0))
  (`self.K2_SetActorLocation` (`KismetMathLibrary.MakeVector` (+ (.x (`self.K2_GetActorLocation` _returnvalue)) (* (`KismetMathLibrary.DegCos` _returnvalue_2) _weapondisplayradius)) (+ (.y (`self.K2_GetActorLocation` _returnvalue)) (* (`KismetMathLibrary.DegSin` _returnvalue_2) _weapondisplayradius)) (.z (`self.K2_GetActorLocation` _returnvalue)))))

(event `Aim Angle update`
  (bind _x (.x (`self.K2_GetActorLocation`)))
  (bind _x_2 (.x (`self.K2_GetActorLocation` (`self.closest_NPC`))))
  (bind _returnvalue (- _x_2 _x))
  (bind _returnvalue_2 (`KismetMathLibrary.DegAtan` (/ (- (.y (`self.K2_GetActorLocation` (`self.closest_NPC`))) (.y (`self.K2_GetActorLocation`))) _returnvalue)))
  ;[1 1 1] 計算並旋轉瞄準角度
  (`self.Update_Closest_NPC`)
  (if (`self.closest_NPC_Exist`)
    (if (!= _returnvalue 0.0)
      (if (> _x_2 _x)
        (`self.K2_SetActorRotation` (`KismetMathLibrary.MakeRotator` 0.0 0.0 _returnvalue_2))
        (else
          (`self.K2_SetActorRotation` (`KismetMathLibrary.MakeRotator` 0.0 0.0 (- _returnvalue_2 180.0))))))))

(event `Update_Closest_NPC`
  ;[1 1 1] 獲取最近敵人(NPC
  (bind _outactors (`GameplayStatics.GetAllActorsOfClass` "/Game/Characters/AI/NPC.NPC_C"))
  (set `self.closest_distance` 2000.0)
  (for _array_element _outactors
    (bind _returnvalue (`self.GetDistanceTo` _array_element))
    (if (<= _returnvalue (`self.closest_distance`))
      (bind _output_get (set `self.closest_distance` _returnvalue))
      (set `self.closest_NPC` _array_element)))
  (set `self.closest_NPC_Exist` (< _output_get 2000.0)))

(fn `init_bullet`
  (params (Direction :type "Transform Structure") (`Life Time` :type "Float (double-precision)")))

(fn `UserConstructionScript`)