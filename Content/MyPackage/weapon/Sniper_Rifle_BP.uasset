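; Sniper rifle weapon actor that follows the third-person player character and automatically fires at the nearest NPC.
; Each tick it snaps to the player, finds the closest NPC within a fixed radius, and yaws toward it using arctangent math.
; A looping BeginPlay delay spawns a batch of bullets every second while a target exists, passing speed, damage, accuracy and range-derived lifetime.
; Its own InitBullet function is an empty stub.
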(event `self.ReceiveBeginPlay`
  (bind _guntest (`self.guntest`))
  (bind _speed (`self.Speed`))
  (if (`self.closest_NPC_Exist`) :!label _label
    (for _ (range 9)
      (bind _returnvalue (`|SpawnActorFromClass` "/Game/MyPackage/weapon/bullet.bullet_C" (`KismetMathLibrary.MakeTransform` (`SceneComponent.K2_GetComponentLocation` _guntest)) "Undefined" "MultiplyWithRoot" null null))
      (`/Game/MyPackage/weapon/bullet.init_bullet` _returnvalue (`SceneComponent.K2_GetComponentRotation` _guntest) (/ (`self.Range`) _speed) _speed (`self.Damage`) (`self.Accuracy`)))
    (`KismetSystemLibrary.Delay` 1.0)
    (goto _label)
    (else
      (`KismetSystemLibrary.Delay` 0.1)
      (goto _label))))

(event `self.ReceiveActorBeginOverlap`
  (params (OtherActor :type "Actor Object Reference"))
  (`self.follow main charater`)
  (`self.Aim Angle update`))

(event `self.ReceiveTick`
  (params (DeltaSeconds :type "Float (single-precision)"))
  (`self.follow main charater`)
  (`self.Aim Angle update`))

(event `follow main charater`
  (bind _returnvalue (`GameplayStatics.GetActorOfClass` "/Game/ThirdPerson/Blueprints/BP_ThirdPersonCharacter.BP_ThirdPersonCharacter_C"))
  (`self.K2_SetActorLocation` (`self.K2_GetActorLocation` _returnvalue)))

(event `Aim Angle update`
  (bind _x (.x (`self.K2_GetActorLocation`)))
  (bind _x_2 (.x (`self.K2_GetActorLocation` (`self.closest_NPC`))))
  (bind _returnvalue (- _x_2 _x))
  (bind _returnvalue_2 (`KismetMathLibrary.DegAtan` (/ (- (.y (`self.K2_GetActorLocation` (`self.closest_NPC`))) (.y (`self.K2_GetActorLocation`))) _returnvalue)))
  ;[1 1 1] 計算並旋轉瞄準角度
  (`self.Update_Closest_NPC`)
  (if (`self.closest_NPC_Exist`)
    (if (!= _returnvalue 0.0)
      (if (> _x_2 _x)
        (`self.K2_SetActorRotation` (`KismetMathLibrary.MakeRotator` 0.0 0.0 (- _returnvalue_2 180.0)))
        (else
          (`self.K2_SetActorRotation` (`KismetMathLibrary.MakeRotator` 0.0 0.0 _returnvalue_2)))))))

(event `Update_Closest_NPC`
  ;[1 1 1] 獲取最近敵人(NPC
  (bind _outactors (`GameplayStatics.GetAllActorsOfClass` "/Game/Characters/AI/NPC.NPC_C"))
  (set `self.closest_distance` 2000.0)
  (for _array_element _outactors
    (bind _returnvalue (`self.GetDistanceTo` _array_element))
    (if (<= _returnvalue (`self.closest_distance`))
      (bind _output_get (set `self.closest_distance` _returnvalue))
      (set `self.closest_NPC` _array_element)))
  (set `self.closest_NPC_Exist` (< _output_get 2000.0)))

(fn `init_bullet`
  (params (Direction :type "Transform Structure") (`Life Time` :type "Float (double-precision)")))

(fn `UserConstructionScript`)